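; BP_EnergyDrink is an energy drink interactable object that changes its sprite when the player character overlaps it.
; It shows the first entry of its Spretes array on BeginPlay.
; Begin and end overlaps with BP_PlayerChar both set the second entry, so the sprite does not revert when the player leaves.
; It contains no pickup or effect logic.
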(event `self.ReceiveBeginPlay`
  (`PaperSpriteComponent.SetSprite` (`self.sprite`) (`|GetArrayItem` (`self.spretes`))))

(event `self.ReceiveActorBeginOverlap`
  (params (OtherActor :type "Actor Object Reference"))
  (cast `/Game/blueprints/BP_PlayerChar` OtherActor)
  (`PaperSpriteComponent.SetSprite` (`self.sprite`) (`|GetArrayItem` (`self.spretes`) 1)))

(event `self.ReceiveActorEndOverlap`
  (params (OtherActor :type "Actor Object Reference"))
  (cast `/Game/blueprints/BP_PlayerChar` OtherActor)
  (`PaperSpriteComponent.SetSprite` (`self.sprite`) (`|GetArrayItem` (`self.spretes`) 1)))

(fn `UserConstructionScript`)